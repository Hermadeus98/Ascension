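; BP_SpaceShip is a player-controlled hovering ship driven by physics forces and Enhanced Input.
; On BeginPlay it adds the IMC_Player mapping context and initializes four hover components with CarMesh.
; The MoveForward input applies force along the mesh's forward vector, scaled by ForwardStrenght and the input value, and prints debug values.
; Forward thrust is the only movement input handled here.
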(event `self.ReceiveBeginPlay`
  (bind _carmesh (`self.CarMesh`))
  (`self.SetupInputMap`)
  (`/Game/Game/Blueprints/BP_HoverComponent.InitComponent` (`self.HoverComponent`) _carmesh)
  (`/Game/Game/Blueprints/BP_HoverComponent.InitComponent` (`self.HoverComponent1`) _carmesh)
  (`/Game/Game/Blueprints/BP_HoverComponent.InitComponent` (`self.HoverComponent2`) _carmesh)
  (`/Game/Game/Blueprints/BP_HoverComponent.InitComponent` (`self.HoverComponent3`) _carmesh))

(event `EnhancedInput|/Game/Game/Blueprints/Inputs/IA_MoveForward`
  (params (ActionValue :type "Float (double-precision)") (ElapsedSeconds :type "Float (double-precision)") (TriggeredSeconds :type "Float (double-precision)") (InputAction :type "InputAction Object Reference" :default "/Game/Game/Blueprints/Inputs/IA_MoveForward.IA_MoveForward"))
  (bind _returnvalue (* (* (`SceneComponent.GetForwardVector` (`self.CarMesh`)) (`self.Forward Strenght`)) ActionValue))
  (:`Triggered`
    (`KismetSystemLibrary.PrintText` (`KismetTextLibrary.Conv_DoubleToText` ActionValue "HalfToEven"))
    (`KismetSystemLibrary.PrintString` (`KismetStringLibrary.Conv_VectorToString` _returnvalue))
    (`PhysicsThreadLibrary.AddForce` (struct) _returnvalue)))

(fn `SetupInputMap`
  (bind _asplayer_controller (cast `PlayerController` (`self.GetController`)))
  (bind _returnvalue (pcsubsystem `EnhancedInputLocalPlayerSubsystem` _asplayer_controller))
  (`/Engine/EditorBlueprintResources/StandardMacros.IsValid` _returnvalue
    (:`Is Valid`
      (`EnhancedInputSubsystemInterface.AddMappingContext` _returnvalue "/Game/Game/Blueprints/Inputs/IMC_Player.IMC_Player" 0 (struct)))))

(fn `UserConstructionScript`)