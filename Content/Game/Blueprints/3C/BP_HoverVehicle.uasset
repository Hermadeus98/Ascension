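; Player-driven physics hover vehicle that accelerates, brakes, steers and boosts through Enhanced Input.
; Four hover components trace for ground, and custom downward gravity applies only when none hit, with overlapped BP_GravityModifier actors overriding its strength.
; Tick ramps acceleration into forward force, sped up by a timed boost and cut faster by braking.
; Smoothed steering drives yaw torque, weakened as acceleration rises, while the mesh parent banks and pitches cosmetically.
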(event `self.ReceiveActorBeginOverlap`
  (params (OtherActor :type "Actor Object Reference"))
  (bind _asbp_gravity_modifier (cast `/Game/Game/Blueprints/GPE/BP_GravityModifier` OtherActor))
  (set `self.Gravity Strength` (`/Game/Game/Blueprints/GPE/BP_GravityModifier.Gravity Strength Modifier` _asbp_gravity_modifier)))

(event `self.ReceiveActorEndOverlap`
  (params (OtherActor :type "Actor Object Reference"))
  (cast `/Game/Game/Blueprints/GPE/BP_GravityModifier` OtherActor)
  (set `self.Gravity Strength` (`self.Default Gravity Strength`)))

(event `self.ReceiveTick`
  (params (DeltaSeconds :type "Float (single-precision)"))
  (bind _space_ship_mesh_parent (`self.Space Ship Mesh Parent`))
  (bind (_relativerotation_roll _relativerotation_pitch _relativerotation_yaw) (`KismetMathLibrary.BreakRotator` (`SceneComponent.RelativeRotation` _space_ship_mesh_parent)))
  (`self.HoverComponentTouchGround`
    (:`true`
      _)
    (:`false`
      (`self.AddGravityStrength`)))
  (`self.ComputeAcceleration` DeltaSeconds (`self.IsAccelerating`))
  (`self.AddAccelerationForce`)
  (set `self.Rotation Percent` (`KismetMathLibrary.Lerp` (`self.Rotation Percent`) (`self.Rotation Input`) (* DeltaSeconds 5.0)))
  (`PrimitiveComponent.AddTorqueInRadians` (`self.Base SpaceShip`) (`KismetMathLibrary.MakeVector` 0.0 0.0 (* (`self.Rotation Percent`) (`KismetMathLibrary.Lerp` (`self.Rotation Strength`) (/ (`self.Rotation Strength`) (`self.Rotation Strength Divider During Acceleration`)) (`self.Acceleration`)))) "None" false)
  (`SceneComponent.K2_SetRelativeRotation` (`self.Space Ship Mesh Parent`) (`KismetMathLibrary.MakeRotator` (* (* (`self.Rotation Percent`) 25.0) (`KismetMathLibrary.Lerp` 2.0 1.0 (`self.Acceleration`)))) false false)
  (if (`self.IsBoosting`)
    (set `self.Boost Elapsed Time` (+ (`self.Boost Elapsed Time`) DeltaSeconds))
    (set `self.Boost Elapsed Time` (`KismetMathLibrary.FClamp` (`self.Boost Elapsed Time`) 0.0 (`self.Boost Duration`)))
    (if (>= (`self.Boost Elapsed Time`) (`self.Boost Duration`))
      (set `self.IsBoosting` false))
    (`KismetSystemLibrary.PrintString` "Stop Boost")
    (`SceneComponent.K2_SetRelativeRotation` _space_ship_mesh_parent (`KismetMathLibrary.MakeRotator` _relativerotation_roll (`KismetMathLibrary.SelectFloat` 10.0 0.0 (`self.IsBoosting`)) _relativerotation_yaw) false false)
    (else
      (set `self.Boost Elapsed Time` 0.0))))

(event `self.ReceiveBeginPlay`
  (`self.SetupInputs`)
  (`self.InitHoverComponents`)
  (set `self.Gravity Strength` (`self.Default Gravity Strength`)))

(event `EnhancedInput|/Game/Game/Blueprints/Inputs/IA_MoveForward`
  (params (ActionValue :type "Float (double-precision)") (ElapsedSeconds :type "Float (double-precision)") (TriggeredSeconds :type "Float (double-precision)") (InputAction :type "InputAction Object Reference" :default "/Game/Game/Blueprints/Inputs/IA_MoveForward.IA_MoveForward"))
  (bind _returnvalue (> ActionValue 0.0))
  (:`Triggered`
    (set `self.IsBraking` (not _returnvalue))
    (set `self.IsAccelerating` _returnvalue))
  (:`Started`
    (if (`self.Boost Input`)
      (`KismetSystemLibrary.PrintString` "Start Boost")
      (set `self.IsBoosting` (> ActionValue 0.0))))
  (:`Canceled`
    (set `self.IsAccelerating` false :!label _label)
    (set `self.IsBoosting` false)
    (`KismetSystemLibrary.PrintString` "Stop Boosting"))
  (:`Completed`
    (goto _label)))

(event `EnhancedInput|/Game/Game/Blueprints/Inputs/IA_MoveRight`
  (params (ActionValue :type "Float (double-precision)") (ElapsedSeconds :type "Float (double-precision)") (TriggeredSeconds :type "Float (double-precision)") (InputAction :type "InputAction Object Reference" :default "/Game/Game/Blueprints/Inputs/IA_MoveRight.IA_MoveRight"))
  (:`Triggered`
    (set `self.Rotation Input` ActionValue))
  (:`Canceled`
    (set `self.Rotation Input` 0.0 :!label _label_2))
  (:`Completed`
    (goto _label_2)))

(event `EnhancedInput|/Game/Game/Blueprints/Inputs/IA_Boost`
  (params (ActionValue :type Boolean) (ElapsedSeconds :type "Float (double-precision)") (TriggeredSeconds :type "Float (double-precision)") (InputAction :type "InputAction Object Reference" :default "/Game/Game/Blueprints/Inputs/IA_Boost.IA_Boost"))
  (:`Triggered`
    (set `self.Boost Input` ActionValue :!label _label_3))
  (:`Canceled`
    (set `self.IsBoosting` false :!label _label_4)
    (goto _label_3))
  (:`Completed`
    (goto _label_4)))

(fn `AddAccelerationForce`
  (`PrimitiveComponent.AddForce` (`self.Base SpaceShip`) (* (* (`SceneComponent.GetForwardVector` (`self.Base SpaceShip`)) (`self.Forward Strength`)) (`self.Acceleration`)) "None" false)
  (return))

(fn `AddGravityStrength`
  (`PrimitiveComponent.AddForceAtLocation` (`self.Base SpaceShip`) (`KismetMathLibrary.MakeVector` 0.0 0.0 (* (`self.Gravity Strength`) -1.0)) (`SceneComponent.K2_GetComponentLocation` (`self.Base SpaceShip`)) "None")
  (return))

(fn `ComputeAcceleration`
  (params (DeltaSecond :type "Float (double-precision)") (Accelerate :type Boolean))
  (bind _accelerationelapsedtime (`self.AccelerationElapsedTime`))
  (bind _acceleration_duration (`self.Acceleration Duration`))
  (bind _accelerationelapsedtime_2 (`self.AccelerationElapsedTime`))
  (bind _acceleration_duration_2 (`self.Acceleration Duration`))
  ;[1 1 1] DECCELERATION
  (if Accelerate
    ;[1 1 1] ACCELERATION
    (set `self.AccelerationElapsedTime` (* (+ (`self.AccelerationElapsedTime`) DeltaSecond) (`KismetMathLibrary.SelectFloat` 2.0 1.0 (`self.IsBoosting`))))
    (set `self.AccelerationElapsedTime` (`KismetMathLibrary.FClamp` _accelerationelapsedtime 0.0 _acceleration_duration_2))
    (set `self.Acceleration` (/ _accelerationelapsedtime _acceleration_duration_2))
    (return)
    (else
      (if (== (`self.IsBraking`) true)
        (set `self.AccelerationElapsedTime` (- (`self.AccelerationElapsedTime`) (* DeltaSecond 10.0)))
        (else
          (set `self.AccelerationElapsedTime` (- (`self.AccelerationElapsedTime`) DeltaSecond))))
      (set `self.AccelerationElapsedTime` (`KismetMathLibrary.FClamp` _accelerationelapsedtime_2 0.0 _acceleration_duration))
      (set `self.Acceleration` (/ _accelerationelapsedtime_2 _acceleration_duration))
      (return))))

(fn `InitHoverComponents`
  (bind _base_spaceship (`self.Base SpaceShip`))
  (`/Game/Game/Blueprints/BP_HoverComponent.InitComponent` (`self.BP_HoverComponent`) _base_spaceship)
  (`/Game/Game/Blueprints/BP_HoverComponent.InitComponent` (`self.BP_HoverComponent1`) _base_spaceship)
  (`/Game/Game/Blueprints/BP_HoverComponent.InitComponent` (`self.BP_HoverComponent2`) _base_spaceship)
  (`/Game/Game/Blueprints/BP_HoverComponent.InitComponent` (`self.BP_HoverComponent3`) _base_spaceship))

(fn `SetupInputs`
  (bind _asplayer_controller (cast `PlayerController` (`self.GetController`)))
  (bind _returnvalue (pcsubsystem `EnhancedInputLocalPlayerSubsystem` _asplayer_controller))
  (`/Engine/EditorBlueprintResources/StandardMacros.IsValid` _returnvalue
    (:`Is Valid`
      (`EnhancedInputSubsystemInterface.AddMappingContext` _returnvalue "/Game/Game/Blueprints/Inputs/IMC_Player.IMC_Player" 0 (struct)))))

(fn `UserConstructionScript`)