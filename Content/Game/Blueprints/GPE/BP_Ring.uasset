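; BP_Ring is a checkpoint ring for hover vehicles, one of a pool that the game mode cycles through at random.
; It registers itself with BP_GameMode on BeginPlay, and Activate only toggles the visibility of its SignActive component.
; When a BP_HoverVehicle overlaps it, it deactivates itself and asks the game mode to activate a random ring.
; The overlap does not check whether the ring is active, so inactive rings also trigger this.
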(event `self.ReceiveBeginPlay`
  (bind _asbp_game_mode (cast `/Game/Game/Blueprints/GameMode/BP_GameMode` (`GameplayStatics.GetGameMode`)))
  (`/Game/Game/Blueprints/GameMode/BP_GameMode.Register Ring` _asbp_game_mode self))

(event `self.ReceiveActorBeginOverlap`
  (params (OtherActor :type "Actor Object Reference"))
  (cast `/Game/Game/Blueprints/3C/BP_HoverVehicle` OtherActor)
  (`KismetSystemLibrary.PrintString` "TRIGGER !")
  (`self.Activate` false)
  (bind _asbp_game_mode (cast `/Game/Game/Blueprints/GameMode/BP_GameMode` (`GameplayStatics.GetGameMode`)))
  (`/Game/Game/Blueprints/GameMode/BP_GameMode.ActivateRandomRing` _asbp_game_mode))

(event `Activate`
  (params (Activation :type Boolean))
  (`SceneComponent.SetVisibility` (`self.Sign_Active`) Activation false))

(fn `UserConstructionScript`)