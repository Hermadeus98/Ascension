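; Game mode that keeps a registry of rings and activates a random one shortly after play begins.
; Rings are added through RegisterRing, and a short BeginPlay delay precedes the first ActivateRandomRing call.
; ActivateRandomRing recurses when its pick equals LastRing, intending to avoid repeats.
; Random is read separately for the check, activation and LastRing assignment, so these can refer to different rings.
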(event `self.ReceiveBeginPlay`
  (`KismetSystemLibrary.Delay` 0.2)
  (`self.ActivateRandomRing`))

(event `Register Ring`
  (params (BP_Ring :type "/Game/Game/Blueprints/GPE/BP_Ring Object Reference"))
  (`BlueprintSetLibrary.Set_Add` (`self.Rings`) BP_Ring))

(fn `ActivateRandomRing`
  (bind _result (`BlueprintSetLibrary.Set_ToArray` (`self.Rings`)))
  (bind _outitem (`KismetArrayLibrary.Array_Random` _result))
  (if (== _outitem (`self.LastRing`))
    (`self.ActivateRandomRing`)
    (else
      (`/Game/Game/Blueprints/GPE/BP_Ring.Activate` _outitem true)
      (set `self.LastRing` _outitem)))
  (return))

(fn `UserConstructionScript`)